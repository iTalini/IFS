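; BP_Fireplace is a fireplace Blueprint with a fuel level bar and a Niagara-style fire effect scaled by intensity.
; On BeginPlay it registers the fuel bar widget from its widget component and sets it to the current fuel level.
; UpdateFireVisual toggles the effect as intensity rises above or drops to zero, then feeds that intensity into curve-scale and velocity-scale effect variables.
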(event `self.ReceiveBeginPlay`
  (`parent.ReceiveBeginPlay`)
  (bind _aswbp_fuel_level_bal (cast `/Game/HUD/Widgets/WBP_FuelLevelBal` (`WidgetComponent.GetWidget` (`self.WidgetBarComponent`))))
  (`self.SetFuelLevelBar` _aswbp_fuel_level_bal)
  (`BasicProgressBar.SetBarPercent` (`self.GetFuelLevelBar`) (`self.GetFuelLevel`)))

(event `self.UpdateFireVisual`
  (params (NewIntensity :type "Float (single-precision)"))
  (bind _fireeffect (`self.FireEffect`))
  (`|ExecutionSequence`
    (:`then_0`
      (if (and (not (`ActorComponent.IsActive` (`self.FireEffect`))) (> NewIntensity 0.0))
        (`ActorComponent.Activate` (`self.FireEffect`) false)
        (elif (and (`ActorComponent.IsActive` (`self.FireEffect`)) (<= NewIntensity 0.0))
          (`ActorComponent.Deactivate` (`self.FireEffect`)))))
    (:`then_1`
      (`NiagaraComponent.SetVariableFloat` _fireeffect (`self.UniformCurveScaleName`) NewIntensity)
      (`NiagaraComponent.SetVariableFloat` _fireeffect (`self.VelocitySpeedScaleName`) NewIntensity))))

(fn `UserConstructionScript`)